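; BP_ForceField is a force field that destroys any actor hitting its sphere and breaks after losing its health.
; Each hit spawns an impact Niagara effect aligned to the surface and restarts a bounce timeline driving a material parameter.
; Health drops only when that timeline finishes, updating the material and destroying the field at zero.
; Show/hide events are empty, and the alpha-fade timeline is unconnected.
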(event OnComponentHit(Sphere)
  (params (HitComponent :type Primitive%20Component%20Object%20Reference) (OtherActor :type Actor%20Object%20Reference) (OtherComp :type Primitive%20Component%20Object%20Reference) (NormalImpulse :type Vector :default "0, 0, 0") (Hit :type Hit%20Result%20Structure%20%28by%20ref%29))
  (bind (_bblockinghit _binitialoverlap _time _distance _location _impactpoint _normal _impactnormal) (Collision|BreakHitResult Hit))
  (bind _sphere (Variables|Default|GetSphere))
  (Actor|DestroyActor OtherActor)
  (Niagara|SpawnSystematLocation "/Game/ForceField/NS_Impact.NS_Impact" _location (Math|Rotator|MakeRotfromX _impactnormal) "3.000000,3.000000,3.000000")
  (bind _bounce_alpha (Timeline|TL_Bounce PlayFromStart)
    (:Update
      (Rendering|Material|SetScalarParameterValueonMaterials _sphere "Bounce Alpha" _bounce_alpha))
    (:Finished
      (bind _output_get (Variables|Default|SetCurrentHealth (- (Variables|Default|GetCurrentHealth) 1)))
      (Development|PrintString "Hello")
      (Rendering|Material|SetScalarParameterValueonMaterials _sphere "CurrentHealth" (Math|Conversions|ToFloat(Integer) _output_get))
      (if (== _output_get 0)
        (Actor|DestroyActor)))))

(event Custom|Show%20ForceField)

(event Custom|Hide%20ForceField)

(event EventBeginPlay)

(fn ConstructionScript)