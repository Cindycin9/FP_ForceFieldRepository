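; BP_Decal is a breakable target cube that shows impact feedback and shatters when its health runs out.
; Each hit spawns glass and impact Niagara effects plus a timed decal, destroys the other actor and plays a bounce timeline.
; Timeline completion decrements DecalHealth into the cube's material, with a large shatter and self-destruction at zero.
; A separate timeline drives material Alpha for ShowDecal and HideDecal, with HideDecal called on BeginPlay.
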(event OnComponentHit(Cube)
  (params (HitComponent :type Primitive%20Component%20Object%20Reference) (OtherActor :type Actor%20Object%20Reference) (OtherComp :type Primitive%20Component%20Object%20Reference) (NormalImpulse :type Vector :default "0, 0, 0") (Hit :type Hit%20Result%20Structure%20%28by%20ref%29))
  (bind (_bblockinghit _binitialoverlap _time _distance _location _impactpoint _normal _impactnormal) (Collision|BreakHitResult Hit))
  (bind _cube (Variables|Default|GetCube))
  (bind _returnvalue (Math|Rotator|MakeRotfromX _impactnormal))
  ;[0.15 0.15 0.15 0.5] ON HIT ( Spawns Niagara system +Destroy actor after health reaches 0)
  (bind _returnvalue_2 (Niagara|SpawnSystematLocation "/Game/Generic_Item_Destruction_FX/Visual_Effects/NiagaraSystem/NS_GlassShatter.NS_GlassShatter" _location _returnvalue "5.000000,5.000000,5.000000"))
  (bind _returnvalue_3 (Niagara|SpawnSystematLocation "/Game/ForceFieldFINALPROTOTYPE/NS_Impact.NS_Impact" _location _returnvalue "2.000000,2.000000,2.000000"))
  ;;[0.2 0.16 0.16] Spawn Decal
  (Rendering|Material|CreateDynamicMaterialInstance "/Game/DECALIMPACTPROTO5/Decay_m_Inst.Decay_m_Inst" "Frame" "None" :!class /Script/Engine.KismetMaterialLibrary)
  (Rendering|Decal|SpawnDecalatLocation "/Game/DECALIMPACTPROTO5/Decay_m.Decay_m" "60.000000,60.000000,60.000000" _location _returnvalue 1e+01)
  (Actor|DestroyActor OtherActor)
  (bind _bounce_alpha (Timeline|Timeline Play)
    (:Update
      (Rendering|Material|SetScalarParameterValueonMaterials _cube "Bounce Alpha" _bounce_alpha))
    (:Finished
      ;;[0.15 0.15 0.15 0.5] Health system
      (bind _output_get (Variables|Default|SetDecalHealth (- (Variables|Default|GetDecalHealth) 1)))
      (Rendering|Material|SetScalarParameterValueonMaterials _cube "DecalHealth" (Math|Conversions|ToFloat(Integer) _output_get))
      ;;[0.15 0.15 0.15 0.5] Once Health reaches 0, Niagara (Shattering/Breaking effect)
      (if (== _output_get 0)
        (Niagara|SpawnSystematLocation "/Game/Generic_Item_Destruction_FX/Visual_Effects/NiagaraSystem/NS_GlassShatter.NS_GlassShatter" _location _returnvalue "100.000000,100.000000,100.000000")
        (Class|NiagaraComponent|SetNiagaraVariableVec3 _returnvalue_2 "" (+ (* _normal "") (* (Transformation|GetActorForwardVector) "")))
        (Actor|DestroyActor)))))

(event Custom|Show%20Decal
  (bind _alpha (Timeline|Timeline_0 Play)
    (:Update
      (Rendering|Material|SetScalarParameterValueonMaterials (Variables|Default|GetCube) "Alpha" _alpha))
    (:Finished
      (CallFunction|HideDecal))))

(event Custom|Hide%20Decal
  (bind _alpha (Timeline|Timeline_0 Reverse)
    (:Update
      (Rendering|Material|SetScalarParameterValueonMaterials (Variables|Default|GetCube) "Alpha" _alpha))
    (:Finished
      (CallFunction|HideDecal))))

(event Collision|EventActorBeginOverlap
  (params (OtherActor :type Actor%20Object%20Reference)))

(event EventTick
  (params (DeltaSeconds :type Float%20%28single-precision%29)))

(event EventBeginPlay
  (CallFunction|HideDecal))

(fn ConstructionScript)