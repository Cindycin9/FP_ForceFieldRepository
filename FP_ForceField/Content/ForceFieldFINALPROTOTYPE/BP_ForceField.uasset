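; BP_ForceField is a destructible force field that destroys any actor hitting it and breaks after losing its health.
; Each hit spawns an impact Niagara effect and plays a bounce timeline driving a material parameter; when that finishes, health drops and damaged materials swap in.
; At zero health it spawns glass Niagara effects and destroys itself.
; The E key flip-flops hide and show, toggling collision and playing or reversing a timeline that animates material alpha and mesh scale.
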(event OnComponentHit(ForcefieldMesh)
  (params (HitComponent :type Primitive%20Component%20Object%20Reference) (OtherActor :type Actor%20Object%20Reference) (OtherComp :type Primitive%20Component%20Object%20Reference) (NormalImpulse :type Vector :default "0, 0, 0") (Hit :type Hit%20Result%20Structure%20%28by%20ref%29))
  (bind (_bblockinghit _binitialoverlap _time _distance _location _impactpoint _normal _impactnormal) (Collision|BreakHitResult Hit))
  (bind _forcefield_mesh (Variables|Default|GetForcefield%20Mesh))
  (bind _returnvalue (Math|Rotator|MakeRotfromX _impactnormal))
  ;[0.15 0.15 0.15 0.5] Upon impact, bullet is destroyed
  (Actor|DestroyActor OtherActor)
  ;[0.15 0.15 0.15 0.5] On impact IMPACT NIAGARA SYSTEM and BOUNCE effect is activated
  (Niagara|SpawnSystematLocation "/Game/ForceFieldFINALPROTOTYPE/NS_Impact.NS_Impact" _location _returnvalue "3.000000,3.000000,3.000000")
  (bind _bounce_alpha (Timeline|TL_Bounce PlayFromStart)
    (:Update
      (Rendering|Material|SetScalarParameterValueonMaterials _forcefield_mesh "Bounce Alpha" _bounce_alpha))
    (:Finished
      ;[0.15 0.15 0.15 0.5] Health of the forcefield
      (bind _output_get (Variables|Default|SetCurrentHealth (- (Variables|Default|GetCurrentHealth) 1)))
      (Rendering|Material|SetScalarParameterValueonMaterials _forcefield_mesh "CurrentHealth" (Math|Conversions|ToFloat(Integer) _output_get))
      ;[0.15 0.15 0.15 0.5] HIT POINTS Upon Hit, Set Material as health status
      (if (== (Variables|Default|GetCurrentHealth) 2)
        (Rendering|Material|SetMaterial (Variables|Default|GetForcefield%20Mesh) 0 "/Game/ForceFieldFINALPROTOTYPE/M_ForceField_Inst_Damaged_2.M_ForceField_Inst_Damaged_2")
        ;[0.15 0.15 0.15 0.5] Once health reaaches 0, Alpha Material deactivates, Glass effect plays and the ForceField is destroyed
        (if (== _output_get 0) :!label _label
          (Niagara|SpawnSystematLocation "/Game/ForceFieldPROTO2/Glass_Niagara.Glass_Niagara" _location _returnvalue "6.000000,6.000000,6.000000")
          (Actor|DestroyActor))
        (elif (== (Variables|Default|GetCurrentHealth) 1)
          (Rendering|Material|SetMaterial (Variables|Default|GetForcefield%20Mesh) 0 "/Game/ForceFieldFINALPROTOTYPE/M_ForceField_Inst_Damaged_1.M_ForceField_Inst_Damaged_1")
          (goto _label)
          (elif (== (Variables|Default|GetCurrentHealth) 0)
            (Rendering|Material|SetMaterial (Variables|Default|GetForcefield%20Mesh) 0 "/Game/ForceFieldFINALPROTOTYPE/M_ForceField_Inst_Damaged_3.M_ForceField_Inst_Damaged_3")
            (Niagara|SpawnSystematLocation "/Game/Generic_Item_Destruction_FX/Visual_Effects/NiagaraSystem/NS_GlassShatter.NS_GlassShatter" _location _returnvalue)
            (goto _label)))))))

(event Custom|Show%20ForceField
  ;[0.15 0.15 0.15 0.5] Appear and Dissapear
  (Collision|SetCollisionEnabled (Variables|Default|GetForcefield%20Mesh) "QueryOnly")
  (CallFunction|ForceFieldGrow))

(event Custom|ForceFieldShrink
  (bind _forcefield_mesh (Variables|Default|GetForcefield%20Mesh))
  ;[0.15 0.15 0.15 0.5] Appear and Dissapear
  (bind (_direction _alpha _scale) (Timeline|Timeline PlayFromStart)
    (:Update
      (Rendering|Material|SetScalarParameterValueonMaterials _forcefield_mesh "Alpha" _alpha)
      (Transformation|SetRelativeScale3D _forcefield_mesh (Math|Conversions|ToVector(Float) _scale)))))

(event Custom|Hide%20ForceField
  ;[0.15 0.15 0.15 0.5] Appear and Dissapear
  (Collision|SetCollisionEnabled (Variables|Default|GetForcefield%20Mesh) "NoCollision")
  (CallFunction|ForceFieldShrink))

(event Custom|ForceFieldGrow
  (bind _forcefield_mesh (Variables|Default|GetForcefield%20Mesh))
  ;[0.15 0.15 0.15 0.5] Appear and Dissapear
  (bind (_direction _alpha _scale) (Timeline|Timeline Reverse)
    (:Update
      (Rendering|Material|SetScalarParameterValueonMaterials _forcefield_mesh "Alpha" _alpha)
      (Transformation|SetRelativeScale3D _forcefield_mesh (Math|Conversions|ToVector(Float) _scale)))))

(event EventBeginPlay
  ;[0.15 0.15 0.15 0.5] Begin Play PlayerController is Enabled
  (Input|EnableInput (Game|GetPlayerController 0) 0))

(event Input|KeyboardEvents|E
  (params (Key :type Key%20Structure :default "None"))
  ;[0.15 0.15 0.15 0.5] Appear and Dissapear
  (:Pressed
    (Utilities|FlowControl|FlipFlop
      (:A
        (CallFunction|HideForceField)
        (Development|PrintString "HideForceField"))
      (:B
        (CallFunction|ShowForceField)
        (Development|PrintString "ShowForceField")))))

(fn ConstructionScript)