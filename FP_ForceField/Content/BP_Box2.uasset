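; BP_Box2 is a destructible Geometry Collection wall that loses health when struck and destroys whatever hits it.
; Each hit spawns a Niagara effect at the impact and restarts a timeline driving a "Bounce Alpha" material parameter.
; When the timeline finishes, it decrements WallHealth, pushes it to the materials, and at zero explodes and destroys the actor.
; Chaos break events swap the material to grimy concrete.
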(event OnChaosBreakEvent(GeometryCollection)
  (params (BreakEvent :type Chaos%20Break%20Event%20Structure%20%28by%20ref%29))
  (Rendering|Material|SetMaterial (Variables|Default|GetGeometryCollection) 0 "/Game/StarterContent/Materials/M_Concrete_Grime.M_Concrete_Grime"))

(event OnComponentHit(GeometryCollection)
  (params (HitComponent :type Primitive%20Component%20Object%20Reference) (OtherActor :type Actor%20Object%20Reference) (OtherComp :type Primitive%20Component%20Object%20Reference) (NormalImpulse :type Vector :default "0, 0, 0") (Hit :type Hit%20Result%20Structure%20%28by%20ref%29))
  (bind (_bblockinghit _binitialoverlap _time _distance _location _impactpoint _normal _impactnormal) (Collision|BreakHitResult Hit))
  (bind _geometrycollection (Variables|Default|GetGeometryCollection))
  (bind _returnvalue (Math|Rotator|MakeRotfromX _impactnormal))
  (Actor|DestroyActor OtherActor)
  (Niagara|SpawnSystematLocation "/Game/Wall1_Niagara.Wall1_Niagara" _location _returnvalue "3.000000,3.000000,3.000000")
  (bind _bounce_alpha (Timeline|Timeline PlayFromStart)
    (:Update
      (Rendering|Material|SetScalarParameterValueonMaterials _geometrycollection "Bounce Alpha" _bounce_alpha))
    (:Finished
      (bind _output_get (Variables|Default|SetWallHealth (- (Variables|Default|GetWallHealth) 1)))
      (Development|PrintString "Hello")
      (Rendering|Material|SetScalarParameterValueonMaterials _geometrycollection "WallHealth" (Math|Conversions|ToFloat(Integer) _output_get))
      (if (== _output_get 0)
        (Niagara|SpawnSystematLocation "/Niagara/DefaultAssets/Templates/Systems/SimpleExplosion.SimpleExplosion" _location _returnvalue "3.000000,3.000000,3.000000")
        (Actor|DestroyActor)
        (Development|PrintString "working")))))

(event EventBeginPlay)

(event Collision|EventActorBeginOverlap
  (params (OtherActor :type Actor%20Object%20Reference)))

(event EventTick
  (params (DeltaSeconds :type Float%20%28single-precision%29)))

(fn ConstructionScript)