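; BP_Cylinder is a prototype force field cylinder that takes damage from impacts and shatters when its health runs out.
; Each component hit destroys the hitting actor, spawns a Niagara impact effect along the surface normal and plays a timeline driving the "Bounce Alpha" material parameter.
; When the timeline finishes, it decrements health and pushes it to the "GlassHealth" material parameter, spawning a glass effect and destroying itself at zero.
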(event OnComponentHit(Cylinder)
  (params (HitComponent :type Primitive%20Component%20Object%20Reference) (OtherActor :type Actor%20Object%20Reference) (OtherComp :type Primitive%20Component%20Object%20Reference) (NormalImpulse :type Vector :default "0, 0, 0") (Hit :type Hit%20Result%20Structure%20%28by%20ref%29))
  (bind (_bblockinghit _binitialoverlap _time _distance _location _impactpoint _normal _impactnormal) (Collision|BreakHitResult Hit))
  (bind _cylinder (Variables|Default|GetCylinder))
  (bind _returnvalue (Math|Rotator|MakeRotfromX _impactnormal))
  ;[0.15 0.15 0.15 0.5] ON HIT ( Spawns Niagara system +Destroy actor after health reaches 0)
  (Actor|DestroyActor OtherActor)
  (Niagara|SpawnSystematLocation "/Game/Wall1_Niagara.Wall1_Niagara" _location _returnvalue "3.000000,3.000000,3.000000")
  (bind _bounce_alpha (Timeline|Timeline PlayFromStart)
    (:Update
      (Rendering|Material|SetScalarParameterValueonMaterials _cylinder "Bounce Alpha" _bounce_alpha))
    (:Finished
      (bind _output_get (Variables|Default|SetCylinderHealth (- (Variables|Default|GetCylinderHealth) 1)))
      (Development|PrintString "Hello")
      (Rendering|Material|SetScalarParameterValueonMaterials _cylinder "GlassHealth" (Math|Conversions|ToFloat(Integer) _output_get))
      (if (== _output_get 0)
        (Niagara|SpawnSystematLocation "/Game/ForceFieldPROTO3/Glass_Niagara.Glass_Niagara" _location _returnvalue "3.000000,3.000000,3.000000")
        (Actor|DestroyActor)
        (Development|PrintString "working")))))

(event EventBeginPlay)

(event Collision|EventActorBeginOverlap
  (params (OtherActor :type Actor%20Object%20Reference)))

(event EventTick
  (params (DeltaSeconds :type Float%20%28single-precision%29)))

(fn ConstructionScript)